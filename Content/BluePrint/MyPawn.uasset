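; Player pawn for a maze game, driven by Enhanced Input through FloatingPawnMovement, with forward/back movement and yaw turning that flips when reversing.
; While Fly is set, Tick runs a pseudo-gravity trace that pushes the pawn down until near the surface.
; IA_Shoot destroys the pawn and has MyMazeGameMode respawn using gathered SpawnPoints and a random MyController; bullet spawning is disconnected.
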(event `self.ReceiveTick`
  (params (DeltaSeconds :type "Float (single-precision)"))
  (if (`self.Fly`)
    (`self.PsevdoGracity`)))

(event `EnhancedInput|/Game/BluePrint/movement/IA_Shoot`
  (params (ActionValue :type Boolean) (ElapsedSeconds :type "Float (double-precision)") (TriggeredSeconds :type "Float (double-precision)") (InputAction :type "InputAction Object Reference" :default "/Game/BluePrint/movement/IA_Shoot.IA_Shoot"))
  (:`Started`
    (bind _asmy_maze_game_mode (cast `MyMazeGameMode` (`GameplayStatics.GetGameMode`)))
    (bind _outactors (`GameplayStatics.GetAllActorsOfClass` "/Game/BluePrint/MyController.MyController_C"))
    (bind _outactors_2 (`GameplayStatics.GetAllActorsOfClass` "/Script/MyProject6.SpawnPoint"))
    (`MyMazeGameMode.SetSpawnPoints` _asmy_maze_game_mode _outactors_2)
    (`self.K2_DestroyActor`)
    (`MyMazeGameMode.SpawnPlayer` _asmy_maze_game_mode (`KismetArrayLibrary.Array_Random` _outactors))))

(event `EnhancedInput|/Game/BluePrint/movement/IA_MoveWS`
  (params (ActionValue :type "Float (double-precision)") (ElapsedSeconds :type "Float (double-precision)") (TriggeredSeconds :type "Float (double-precision)") (InputAction :type "InputAction Object Reference" :default "/Game/BluePrint/movement/IA_MoveWS.IA_MoveWS"))
  (bind (_returnvalue_roll _returnvalue_pitch _returnvalue_yaw) (`KismetMathLibrary.BreakRotator` (`self.GetControlRotation`)))
  (:`Triggered`
    (set `self.MoveWS?` ActionValue :!label _label)
    (`PawnMovementComponent.AddInputVector` (`self.FloatingPawnMovement`) (* (`KismetMathLibrary.GetForwardVector` (`KismetMathLibrary.MakeRotator` _returnvalue_roll 0.0 _returnvalue_yaw)) (* ActionValue (`self.MoveSpeed`))) false))
  (:`Started`
    (goto _label))
  (:`Completed`
    (set `self.MoveWS?` 0.0)))

(event `EnhancedInput|/Game/BluePrint/movement/IA_MoveAD`
  (params (ActionValue :type "Float (double-precision)") (ElapsedSeconds :type "Float (double-precision)") (TriggeredSeconds :type "Float (double-precision)") (InputAction :type "InputAction Object Reference" :default "/Game/BluePrint/movement/IA_MoveAD.IA_MoveAD"))
  (:`Triggered`
    (if (== (`self.MoveWS?`) -1.0)
      (`self.AddControllerYawInput` (* ActionValue 0.5))
      (else
        (`self.AddControllerYawInput` (* ActionValue -0.5))))))

(fn `PsevdoGracity`
  (bind _scene (`self.Scene`))
  (bind _returnvalue (`SceneComponent.K2_GetComponentLocation` _scene))
  (bind _returnvalue_2 (* (`KismetMathLibrary.GetUpVector` (`SceneComponent.K2_GetComponentRotation` _scene)) (-1.0 -1.0 -1.0)))
  (bind _outhit (`KismetSystemLibrary.LineTraceSingle` :`Start` _returnvalue :`End` (+ _returnvalue (* _returnvalue_2 10000.0)) :`TraceChannel` "TraceTypeQuery1" :`DrawDebugType` "ForDuration"))
  (if (> (`.Distance` (`GameplayStatics.BreakHitResult` _outhit)) 10.0)
    (`PawnMovementComponent.AddInputVector` (`self.FloatingPawnMovement`) (* _returnvalue_2 50.0) false)
    (else
      (set `self.Fly` false))))

(fn `UserConstructionScript`)