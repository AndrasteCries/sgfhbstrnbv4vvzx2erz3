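; Game mode for a maze game that holds player spawning until the procedural maze has finished generating.
; Tick polls MyMazeGenerator through a Gate; once generation completes, it passes the MazeGeneratorCell actors to SetSpawnPoints, spawns a random MyController's player and closes the gate.
; PostLogin spawns each joining player once the cached Generated flag is true, otherwise retrying through a one-second Delay loop.
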(event `self.ReceiveBeginPlay`)

(event `self.ReceiveTick`
  (params (DeltaSeconds :type "Float (single-precision)"))
  (`/Engine/EditorBlueprintResources/StandardMacros.Gate` false :!label _label
    (:`Exit`
      (bind _returnvalue (`GameplayStatics.GetActorOfClass` "/Game/BluePrint/MyMazeGenerator.MyMazeGenerator_C"))
      (bind _asmy_maze_generator (cast `/Game/BluePrint/MyMazeGenerator` _returnvalue))
      (bind _returnvalue_2 (`MazeGenerator.GetMazeGenerated` _asmy_maze_generator))
      (set `self.Generated` _returnvalue_2)
      (if _returnvalue_2
        (bind _outactors (`GameplayStatics.GetAllActorsOfClass` "/Script/MyProject6.MazeGeneratorCell"))
        (`self.SetSpawnPoints` _outactors)
        (bind _outactors_2 (`GameplayStatics.GetAllActorsOfClass` "/Game/BluePrint/MyController.MyController_C"))
        (bind (_outitem _outindex) (`KismetArrayLibrary.Array_Random` _outactors_2))
        (`KismetSystemLibrary.PrintString` (`KismetStringLibrary.Conv_IntToString` _outindex))
        (`self.SpawnPlayer` _outitem)
        (goto _label :!via `Close`)
        (else
          (`KismetSystemLibrary.PrintString` "Hello"))))))

(event `self.K2_PostLogin`
  (params (NewPlayer :type "PlayerController Object Reference"))
  (if (`self.Generated`) :!label _label_2
    (`self.SpawnPlayer` NewPlayer)
    (else
      (`KismetSystemLibrary.Delay` 1.0)
      (goto _label_2))))

(fn `UserConstructionScript`)